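; BP_SavedCustomizations holds a Data array of named character customization profiles, with lookup functions for them.
; GetCustomizationByProfileName scans the array for a matching ProfileName and returns that entry with its index, or an index of -1 when none matches.
; GetProfileNames collects the ProfileName of every entry into a list.
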(fn GetCustomizationbyProfileName
  (params (ProfileName :type String))
  (for (_array_element _array_index) (Variables|Default|GetData)
    (if (Utilities|Enum|Equal(Enum) ProfileName (Utilities|Struct|BreakSSaveData _array_element))
      (return _array_element _array_index)))
  (return "" -1))

(fn GetProfileNames
  (for _array_element (Variables|Default|GetData)
    (Utilities|Array|Add (LocalVariables|GetProfileNames) (Utilities|Struct|BreakSSaveData _array_element)))
  (return (LocalVariables|GetProfileNames)))